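; Lane actor for an endless road-crossing game that randomly becomes road, water, railroad or long grass.
; On BeginPlay it sets both meshes, offsets its SpawnPoint by the scaled mesh width, and spawns a Vehicle_spawner on a random side with the lane's identity.
; A player overlapping its trigger while moving in negative X asks LaneSpawner for a new lane.
; An edge handler destroys obstacles that pass the opposite spawn point.
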(event `self.ReceiveBeginPlay`
  (`self.SetMeshes`)
  (`self.CreateVehicleSpawner`))

(event `self.TriggerZone.OnComponentBeginOverlap`
  (params (OverlappedComponent :type "PrimitiveComponent Object Reference") (OtherActor :type "Actor Object Reference") (OtherComp :type "PrimitiveComponent Object Reference") (OtherBodyIndex :type Integer) (bFromSweep :type Boolean) (SweepResult :type "HitResult Structure (by ref)"))
  (bind _returnvalue_x (`KismetMathLibrary.BreakVector` (`Pawn.GetLastMovementInputVector` (`GameplayStatics.GetPlayerPawn` 0))))
  (cast `/Game/blueprints/player_bp` OtherActor)
  (if (< _returnvalue_x 0.0)
    (`/Game/blueprints/lane_spawner.Spawn Lane at Newest Location` (`self.lane_spawner`) false)))

(event `handle drive past edge`
  (params (left :type Boolean) (location :type "Vector Structure") (obstacle :type "/Game/blueprints/truck_bp Object Reference"))
  (bind (_returnvalue_x _returnvalue_y) (`KismetMathLibrary.BreakVector` (`SceneComponent.K2_GetComponentLocation` (`self.LeftSpawnPoint`))))
  (bind (_returnvalue_x_2 _returnvalue_y_2) (`KismetMathLibrary.BreakVector` (`SceneComponent.K2_GetComponentLocation` (`self.RightSpawnPoint`))))
  (if left
    (if (<= location_Y _returnvalue_y_2)
      (`self.K2_DestroyActor` obstacle))
    (elif (> location_Y _returnvalue_y)
      (`self.K2_DestroyActor` obstacle))))

(fn `CreateVehicleSpawner`
  (bind _vehicle_spawner (`self.vehicle_spawner`))
  (bind _vehicle_spawner_2 (`self.vehicle_spawner`))
  (bind _returnvalue (`|SpawnActorFromClass` "/Game/blueprints/vehicle_spawner.vehicle_spawner_C" (`KismetMathLibrary.MakeTransform` (0.0 0.0 0.0)) "Undefined" "OverrideRootScale" null null))
  (bind _output_get (set `self.vehicle_spawner` _returnvalue))
  (if (`KismetMathLibrary.Conv_IntToBool` (`KismetMathLibrary.RandomIntegerInRange` 0 1))
    (set `/Game/blueprints/vehicle_spawner.spawn_location` (`SceneComponent.K2_GetComponentLocation` (`self.LeftSpawnPoint`)) _vehicle_spawner_2)
    (set `/Game/blueprints/vehicle_spawner.left` true _vehicle_spawner_2)
    (else
      (set `/Game/blueprints/vehicle_spawner.spawn_location` (`SceneComponent.K2_GetComponentLocation` (`self.RightSpawnPoint`)) _vehicle_spawner)
      (set `/Game/blueprints/vehicle_spawner.left` false _vehicle_spawner)))
  (set `/Game/blueprints/vehicle_spawner.identity` (`self.identity`) _output_get)
  (set `/Game/blueprints/vehicle_spawner.current_lane` self _output_get)
  (`/Game/blueprints/vehicle_spawner.create spawn timer` _output_get))

(fn `Generate Identity`
  (bind _result (`/Engine/EditorBlueprintResources/StandardMacros.DecrementInt` (`self.num_types`))
    (:`  `
      (bind _output_get (set `self.identity` (`KismetMathLibrary.RandomIntegerInRange` 0 _result)))
      (`KismetSystemLibrary.PrintString` (`KismetStringLibrary.Conv_IntToString` _output_get)))))

(fn `SetMeshes`
  (bind _returnvalue (select `int` (`self.identity`) :`0` "/Game/roads/1road-marked.1road-marked" :`1` "/Game/roads/1lane_water.1lane_water" :`2` "/Game/roads/railroad.railroad" :`3` "/Game/roads/longgrass.longgrass" :!type "StaticMesh Object Reference"))
  (`self.Generate Identity`)
  (`StaticMeshComponent.SetStaticMesh` (`self.StaticMesh`) _returnvalue)
  (`StaticMeshComponent.SetStaticMesh` (`self.StaticMesh2`) _returnvalue)
  (`self.SetSpawnPoint`))

(fn `SetSpawnPoint`
  (bind _returnvalue_x (`KismetMathLibrary.BreakVector` (`SceneComponent.K2_GetComponentLocation` (`self.StaticMesh`))))
  (bind (_returnvalue_min _returnvalue_max) (break `Box` (`StaticMesh.GetBoundingBox` (`StaticMeshComponent.StaticMesh` (`self.StaticMesh`)))))
  (bind _returnvalue_x_2 (`KismetMathLibrary.BreakVector` (- _returnvalue_max _returnvalue_min)))
  (bind _returnvalue (- _returnvalue_x (* _returnvalue_x_2 (`self.lane_scale`))))
  (`KismetSystemLibrary.PrintString` (`KismetStringLibrary.Conv_DoubleToString` _returnvalue_x))
  (`KismetSystemLibrary.PrintString` (`KismetStringLibrary.Conv_DoubleToString` _returnvalue))
  (`SceneComponent.K2_SetWorldLocation` (`self.SpawnPoint`) (`KismetMathLibrary.MakeVector` _returnvalue) false false))

(fn `UserConstructionScript`)