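; Lane spawner actor that builds a continuous strip of scaled lanes, clearing existing Lane_bp actors at BeginPlay, then laying initial grass (Lane_bp_2) followed by roads (Lane_bp).
; Each lane's SpawnPoint component sets where the next one spawns, chaining them end to end.
; Every lane receives a reference to the spawner.
; The looping timer for interval spawning is disconnected, so this actor only self-triggers the initial build.
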(event `self.ReceiveBeginPlay`
  (`self.SpawnInitialLanes`))

(event `Spawn lanes by intervals`
  (`self.Spawn Lane at Newest Location` false))

(fn `Spawn Lane at Newest Location`
  (params (InitialBase :type Boolean))
  (`self.SpawnLane` (`self.newest spawn point`) InitialBase))

(fn `SpawnInitialLanes`
  (`|ExecutionSequence`
    (:`then_0`
      (bind _outactors (`GameplayStatics.GetAllActorsOfClass` "/Game/blueprints/lane_bp.lane_bp_C"))
      (for _array_element _outactors
        (`self.K2_DestroyActor` _array_element)))
    (:`then_1`
      (for _ (range (+ (`self.inital_grass_num`) 1))
        (if (== (`self.newest spawn point`) (0.0 0.0 0.0))
          (`self.SpawnLane` (`self.initial location`) true)
          (else
            (`self.Spawn Lane at Newest Location` true)))))
    (:`then_2`
      (for _ (range (+ (`self.num_roads_on_screen`) 1))
        (`self.Spawn Lane at Newest Location` false)))))

(fn `SpawnLane`
  (params (SpawnLocation :type "Vector Structure") (InitialBase :type Boolean))
  (bind _returnvalue (* (`self.lane_scale`) (`KismetMathLibrary.MakeVector` 1.0 1.0 1.0)))
  (if InitialBase
    (bind _returnvalue_2 (`|SpawnActorFromClass` "/Game/blueprints/lane_bp_2.lane_bp_2_C" (`KismetMathLibrary.MakeTransform` SpawnLocation (struct) _returnvalue) "Undefined" "OverrideRootScale" null null))
    (set `self.newest spawn point` (`SceneComponent.K2_GetComponentLocation` (`/Game/blueprints/lane_bp_2.SpawnPoint` _returnvalue_2)))
    (set `/Game/blueprints/lane_bp_2.lane_spawner` self _returnvalue_2)
    (else
      (bind _returnvalue_3 (`|SpawnActorFromClass` "/Game/blueprints/lane_bp.lane_bp_C" (`KismetMathLibrary.MakeTransform` SpawnLocation (struct) _returnvalue) "Undefined" "OverrideRootScale" null null))
      (set `self.newest spawn point` (`SceneComponent.K2_GetComponentLocation` (`/Game/blueprints/lane_bp.SpawnPoint` _returnvalue_3)))
      (set `/Game/blueprints/lane_bp.lane_spawner` self _returnvalue_3))))

(fn `UserConstructionScript`)