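; Vehicle spawner actor that spawns left-facing Truck_bp vehicles at its spawn location for a lane.
; A looping timer, started by a custom event rather than BeginPlay, gives an even chance of spawning on each tick of the timer.
; The construction script rolls one random speed per spawner, which each truck receives along with the current lane and a mesh selected by Identity.
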(event `self.ReceiveBeginPlay`)

(event `create spawn timer`
  (`KismetSystemLibrary.K2_SetTimerDelegate` (delegate `spawn vehicle randomly`) 5.0 true))

(event `spawn vehicle randomly`
  (if (`KismetMathLibrary.Conv_IntToBool` (`KismetMathLibrary.RandomIntegerInRange` 0 1))
    (`self.SpawnVehicle` (`self.spawn_location`))))

(event `self.ReceiveTick`
  (params (DeltaSeconds :type "Float (single-precision)")))

(fn `SetRandomVehicleSpeed`
  (set `self.vehicle_speed` (`KismetMathLibrary.Conv_IntToDouble` (`KismetMathLibrary.RandomIntegerInRange` 100 500))))

(fn `SpawnVehicle`
  (params (SpawnPoint :type "Vector Structure"))
  (bind _returnvalue (`|SpawnActorFromClass` "/Game/blueprints/truck_bp.truck_bp_C" (`KismetMathLibrary.MakeTransform` SpawnPoint) "Undefined" "OverrideRootScale" null null))
  (set `/Game/blueprints/truck_bp.direction` (`self.left`) _returnvalue)
  (`/Game/blueprints/truck_bp.SetMeshDirection` _returnvalue)
  (`/Game/blueprints/truck_bp.SetMesh` _returnvalue (select `int` (`self.identity`) :`0` "/Game/vehicles/fedex.fedex" :`1` "/Game/terrain/rock.rock" :`2` "/Game/vehicles/train.train" :!type "StaticMesh Object Reference"))
  (set `/Game/blueprints/truck_bp.current_lane` (`self.current_lane`) _returnvalue)
  (set `/Game/blueprints/truck_bp.Speed` (`self.vehicle_speed`) _returnvalue))

(fn `UserConstructionScript`
  (`self.SetRandomVehicleSpeed`))