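; Truck obstacle that drives along a lane and kills the player when its mesh hits them.
; Each Tick moves it along world Y according to Direction and Speed, applies a Gravity-scaled Z offset, then lets CurrentLane handle driving past the edge.
; Only the Direction-true move and the gravity offset use sweep.
; Helper functions swap the mesh and rotate the actor 180 degrees when Direction is false.
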(event `self.ReceiveTick`
  (params (DeltaSeconds :type "Float (single-precision)"))
  (`self.Drive` DeltaSeconds)
  (`self.K2_AddActorLocalOffset` (`KismetMathLibrary.MakeVector` 0.0 0.0 (* DeltaSeconds (`self.gravity`))) true)
  (`/Game/blueprints/lane_bp.handle drive past edge` (`self.current_lane`) (`self.direction`) (`self.K2_GetActorLocation`) self))

(event `self.TruckMesh.OnComponentHit`
  (params (HitComponent :type "PrimitiveComponent Object Reference") (OtherActor :type "Actor Object Reference") (OtherComp :type "PrimitiveComponent Object Reference") (NormalImpulse :type "Vector Structure") (Hit :type "HitResult Structure (by ref)"))
  (bind _asplayer_bp (cast `/Game/blueprints/player_bp` OtherActor))
  (`/Game/blueprints/player_bp.player die` _asplayer_bp))

(fn `Drive`
  (params (delta_seconds :type "Float (double-precision)"))
  (bind _returnvalue (* delta_seconds (`self.Speed`)))
  (if (`self.direction`)
    (`self.K2_AddActorWorldOffset` (`KismetMathLibrary.MakeVector` 0.0 (* _returnvalue -1.0)) true)
    (else
      (`self.K2_AddActorWorldOffset` (`KismetMathLibrary.MakeVector` 0.0 _returnvalue)))))

(fn `SetMesh`
  (params (mesh :type "StaticMesh Object Reference"))
  (`StaticMeshComponent.SetStaticMesh` (`self.TruckMesh`) mesh))

(fn `SetMeshDirection`
  (if (not (`self.direction`))
    (`self.K2_SetActorRotation` (struct :`Yaw` 180.0))))

(fn `UserConstructionScript`)