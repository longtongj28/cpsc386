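; Player pawn Blueprint with hand-rolled movement and a simple death state.
; Move axes add input along the actor's forward and right vectors scaled by MaxSpeed, which Tick consumes as a swept, delta-time-scaled offset while alive.
; The playerdie event tips the mesh 90 degrees and sets Dead, stopping movement.
; Jump is a one-shot upward offset that nothing here calls, and the gravity offset is disconnected.
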(event `self.ReceiveBeginPlay`)

(event `self.ReceiveTick`
  (params (DeltaSeconds :type "Float (single-precision)"))
  (if (not (`self.dead`))
    (bind _returnvalue (`self.ConsumeMovementInputVector`))
    (`self.K2_AddActorLocalOffset` (* _returnvalue DeltaSeconds) true)))

(event `InputAxis|MoveRight`
  (params (AxisValue :type "Float (single-precision)"))
  (`self.AddMovementInput` (`self.GetActorRightVector`) (* AxisValue (`self.max_speed`))))

(event `InputAxis|MoveForward`
  (params (AxisValue :type "Float (single-precision)"))
  (`self.AddMovementInput` (`self.GetActorForwardVector`) (* AxisValue (`self.max_speed`))))

(event `player die`
  (if (not (`self.dead`))
    (`SceneComponent.K2_SetRelativeRotation` (`self.StaticMesh`) (struct :`Roll` 90.0) false false)
    (set `self.dead` true)))

(fn `Jump`
  (`self.K2_AddActorLocalOffset` (`KismetMathLibrary.MakeVector` 0.0 0.0 (`self.jump_speed`)) true))

(fn `UserConstructionScript`)