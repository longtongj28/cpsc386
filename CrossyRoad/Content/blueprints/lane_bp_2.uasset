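; Lane actor that asks its LaneSpawner for a new lane as the player advances across it.
; On BeginPlay, SetMeshes positions SpawnPoint one scaled mesh-bounds length along negative X from the mesh.
; TriggerZone overlap by player_bp spawns at the newest location only when the last movement input points toward negative X.
; GenerateIdentity picks a random lane type index but is not called in this graph.
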(event `self.ReceiveBeginPlay`
  (`self.SetMeshes`))

(event `self.TriggerZone.OnComponentBeginOverlap`
  (params (OverlappedComponent :type "PrimitiveComponent Object Reference") (OtherActor :type "Actor Object Reference") (OtherComp :type "PrimitiveComponent Object Reference") (OtherBodyIndex :type Integer) (bFromSweep :type Boolean) (SweepResult :type "HitResult Structure (by ref)"))
  (bind _returnvalue_x (`KismetMathLibrary.BreakVector` (`Pawn.GetLastMovementInputVector` (`GameplayStatics.GetPlayerPawn` 0))))
  (cast `/Game/blueprints/player_bp` OtherActor)
  (if (< _returnvalue_x 0.0)
    (`/Game/blueprints/lane_spawner.Spawn Lane at Newest Location` (`self.lane_spawner`) false)
    (`KismetSystemLibrary.PrintString` "cross spawn point")))

(fn `Generate Identity`
  (bind _result (`/Engine/EditorBlueprintResources/StandardMacros.DecrementInt` (`self.num_types`))
    (:`  `
      (bind _output_get (set `self.identity` (`KismetMathLibrary.RandomIntegerInRange` 0 _result)))
      (`KismetSystemLibrary.PrintString` (`KismetStringLibrary.Conv_IntToString` _output_get)))))

(fn `SetMeshes`
  (`self.SetSpawnPoint`))

(fn `SetSpawnPoint`
  (bind _returnvalue_x (`KismetMathLibrary.BreakVector` (`SceneComponent.K2_GetComponentLocation` (`self.StaticMesh`))))
  (bind (_returnvalue_min _returnvalue_max) (break `Box` (`StaticMesh.GetBoundingBox` (`StaticMeshComponent.StaticMesh` (`self.StaticMesh`)))))
  (bind _returnvalue_x_2 (`KismetMathLibrary.BreakVector` (- _returnvalue_max _returnvalue_min)))
  (bind _returnvalue (- _returnvalue_x (* _returnvalue_x_2 (`self.lane_scale`))))
  (`KismetSystemLibrary.PrintString` (`KismetStringLibrary.Conv_DoubleToString` _returnvalue_x))
  (`KismetSystemLibrary.PrintString` (`KismetStringLibrary.Conv_DoubleToString` _returnvalue))
  (`SceneComponent.K2_SetWorldLocation` (`self.SpawnPoint`) (`KismetMathLibrary.MakeVector` _returnvalue) false false))

(fn `UserConstructionScript`)